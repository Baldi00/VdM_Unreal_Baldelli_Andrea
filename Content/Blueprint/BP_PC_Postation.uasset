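; Interactive PC workstation prop whose screens switch on and off when used.
; BeginPlay creates dynamic material instances from a default material, one shared by two screen slots and one for the case slot.
; Interact plays a button sound and uses a FlipFlop to toggle the screens between glowing white and unlit black.
; StartHovering and StopHovering add or clear a faint emissive highlight on the case.
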(event EventStopHovering
  (Rendering|Material|SetScalarParameterValue (Variables|Default|GetCaseMaterial) "Emission" 0.0 :!class /Script/Engine.MaterialInstanceDynamic))

(event EventInteract
  (bind _screenmaterial (Variables|Default|GetScreenMaterial))
  (bind _screenmaterial_2 (Variables|Default|GetScreenMaterial))
  (Audio|PlaySound2D "/Game/Sounds/FX/PcButtonPressed.PcButtonPressed" 1.0 1.0 0.0 0 0)
  (Utilities|FlowControl|FlipFlop
    (:A
      (Rendering|Material|SetScalarParameterValue _screenmaterial_2 "Emission" 2.0 :!class /Script/Engine.MaterialInstanceDynamic)
      (Rendering|Material|SetVectorParameterValue _screenmaterial_2 "BaseColor" "(R=1.000000,G=1.000000,B=1.000000,A=1.000000)" :!class /Script/Engine.MaterialInstanceDynamic))
    (:B
      (Rendering|Material|SetScalarParameterValue _screenmaterial "Emission" 0.0 :!class /Script/Engine.MaterialInstanceDynamic)
      (Rendering|Material|SetVectorParameterValue _screenmaterial "BaseColor" "(R=0.000000,G=0.000000,B=0.000000,A=1.000000)" :!class /Script/Engine.MaterialInstanceDynamic))))

(event EventBeginPlay
  (bind _sm_pc_postation (Variables|Default|GetSM_PC_Postation))
  (Utilities|FlowControl|Sequence
    (:then_0
      (bind _returnvalue (Rendering|Material|CreateDynamicMaterialInstance "/Game/Art/MaterialLibrary/M_DefaultMaterial.M_DefaultMaterial" "None" "None" :!class /Script/Engine.KismetMaterialLibrary))
      (Variables|Default|SetScreenMaterial _returnvalue)
      (Rendering|Material|SetMaterial _sm_pc_postation 5 (Variables|Default|GetScreenMaterial))
      (Rendering|Material|SetMaterial _sm_pc_postation 13 (Variables|Default|GetScreenMaterial)))
    (:then_1
      (bind _returnvalue_2 (Rendering|Material|CreateDynamicMaterialInstance (Variables|Default|GetSM_PC_Postation) 9 "/Game/Art/MaterialLibrary/M_DefaultMaterial.M_DefaultMaterial" "None" :!class /Script/Engine.PrimitiveComponent))
      (Variables|Default|SetCaseMaterial _returnvalue_2))))

(event EventStartHovering
  (Rendering|Material|SetScalarParameterValue (Variables|Default|GetCaseMaterial) "Emission" 0.025 :!class /Script/Engine.MaterialInstanceDynamic))

(fn ConstructionScript)