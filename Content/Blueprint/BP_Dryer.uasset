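; BP_Dryer is an interactable air dryer prop that lights up for a few seconds when used.
; At BeginPlay it creates a dynamic material on the dryer mesh, and hover events toggle a faint emission highlight through it.
; Interact turns on a spot and point light unless already running, then a one-shot timer switches them off and clears the running flag.
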(event Custom|StopAirDryer
  (Rendering|SetVisibility (Variables|Default|GetSpotLight) false false)
  (Rendering|SetVisibility (Variables|Default|GetPointLight) false false)
  (Variables|Default|SetIsRunning false))

(event EventStopHovering
  (Rendering|Material|SetScalarParameterValue (Variables|Default|GetAirDryerMaterial) "Emission" 0.0 :!class /Script/Engine.MaterialInstanceDynamic))

(event EventBeginPlay
  (bind _returnvalue (Rendering|Material|CreateDynamicMaterialInstance (Variables|Default|GetEnvironment_AirDryer) 0 "/Game/Art/MaterialLibrary/MI_DefaultMaterial_White.MI_DefaultMaterial_White" "None" :!class /Script/Engine.PrimitiveComponent))
  (Variables|Default|SetAirDryerMaterial _returnvalue))

(event EventInteract
  (if (not (Variables|Default|GetIsRunning))
    (Variables|Default|SetIsRunning true)
    (Rendering|SetVisibility (Variables|Default|GetSpotLight) true false)
    (Rendering|SetVisibility (Variables|Default|GetPointLight) true false)
    (Utilities|Time|SetTimerbyEvent (delegate Custom|StopAirDryer) 5.0)))

(event EventStartHovering
  (Rendering|Material|SetScalarParameterValue (Variables|Default|GetAirDryerMaterial) "Emission" 0.025 :!class /Script/Engine.MaterialInstanceDynamic))

(fn ConstructionScript)