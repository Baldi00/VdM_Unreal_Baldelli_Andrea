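; BP_Door is an interactive door actor that swings open and closed and glows faintly while hovered.
; BeginPlay creates a dynamic material on the Door component, caches the starting rotation, then applies InitialRotation as a yaw offset.
; Interact flip-flops the RotateAnimation timeline forward and back, lerping yaw between InitialRotation and EndRotation relative to that cached rotation.
; StartHovering and StopHovering toggle the material's Emission parameter as a highlight.
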(event EventStopHovering
  (Rendering|Material|SetScalarParameterValue (Variables|Default|GetDoorMaterial) "Emission" 0.0 :!class /Script/Engine.MaterialInstanceDynamic))

(event EventInteract
  (Utilities|FlowControl|FlipFlop
    (:A
      (bind _rotation (Timeline|RotateAnimation Play)
        (:Update
          (Transformation|SetActorRotation (Math|Rotator|MakeRotator 0.0 0.0 (+ (Math|Float|Lerp (Variables|Default|GetInitialRotation) (Variables|Default|GetEndRotation) _rotation) (.yaw (Variables|Default|GetInitialActorRotation))))))))
    (:B
      (Timeline|RotateAnimation Reverse))))

(event EventBeginPlay
  (Utilities|FlowControl|Sequence
    (:then_0
      (bind _returnvalue (Rendering|Material|CreateDynamicMaterialInstance (Variables|Default|GetDoor) 0 "/Game/Art/MaterialLibrary/MI_DefaultMaterial_White.MI_DefaultMaterial_White" "None" :!class /Script/Engine.PrimitiveComponent))
      (Variables|Default|SetDoorMaterial _returnvalue))
    (:then_1
      (Variables|Default|SetInitialActorRotation (Transformation|GetActorRotation)))
    (:then_2
      (Transformation|SetActorRotation (Math|Rotator|MakeRotator 0.0 0.0 (+ (Variables|Default|GetInitialRotation) (.yaw (Variables|Default|GetInitialActorRotation))))))))

(event EventStartHovering
  (Rendering|Material|SetScalarParameterValue (Variables|Default|GetDoorMaterial) "Emission" 0.05 :!class /Script/Engine.MaterialInstanceDynamic))

(fn ConstructionScript)