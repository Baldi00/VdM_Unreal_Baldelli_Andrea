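; Interactable drink dispenser that highlights on hover and spawns a BP_Drink when used.
; Hover events toggle emission on a dynamic material, and the construction script writes the display name to its text.
; Interact plays a beep, spawns the drink at the emitter, then randomizes its rotation, launch force and fully saturated color.
; When IsMagic is set, the drink also glows in that color.
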(event EventStopHovering
  (Rendering|Material|SetScalarParameterValue (Variables|Default|GetDispenserMaterial) "Emission" 0.0 :!class /Script/Engine.MaterialInstanceDynamic))

(event EventBeginPlay
  (bind _returnvalue (Rendering|Material|CreateDynamicMaterialInstance (Variables|Default|GetDispenser) 0 "/Game/Art/MaterialLibrary/M_DefaultMaterial.M_DefaultMaterial" "None" :!class /Script/Engine.PrimitiveComponent))
  (Variables|Default|SetDispenserMaterial _returnvalue))

(event EventInteract
  (bind _returnvalue (Math|Random|RandomUnitVector))
  (bind _returnvalue_2 (* _returnvalue 3.6e+02))
  (Audio|PlaySound2D "/Game/Sounds/FX/DispenserBip.DispenserBip" 1.0 1.0 0.0 0 0)
  (bind _returnvalue_3 (Game|SpawnActorfromClass "/Game/Blueprint/BP_Drink.BP_Drink_C" (Transformation|GetWorldTransform (Variables|Default|GetEmitter)) "Undefined" "MultiplyWithRoot" 0 0))
  (Variables|Default|SetCurrentSpawnedDrink (Variables|/Game/Blueprint/BP_Drink.BP_Drink_C|GetDrink _returnvalue_3))
  (Utilities|FlowControl|Sequence
    (:then_0
      (Transformation|SetWorldRotation (Variables|Default|GetCurrentSpawnedDrink) (Math|Rotator|MakeRotator (.x _returnvalue_2) (.y _returnvalue_2) (.z _returnvalue_2)) false false))
    (:then_1
      (Physics|AddForce (Variables|Default|GetCurrentSpawnedDrink) (* (Math|Vector|VectorGetAbs (Math|Random|RandomUnitVector)) 5e+05) "None" false))
    (:then_2
      (bind _returnvalue_4 (Rendering|Material|CreateDynamicMaterialInstance (Variables|Default|GetCurrentSpawnedDrink) 0 "/Game/Art/MaterialLibrary/M_DefaultMaterial.M_DefaultMaterial" "None" :!class /Script/Engine.PrimitiveComponent))
      (bind _randomcolor (CallFunction|GetRandomColor))
      (Variables|Default|SetCurrentRandomColor _randomcolor)
      (Rendering|Material|SetVectorParameterValue _returnvalue_4 "BaseColor" (Variables|Default|GetCurrentRandomColor) :!class /Script/Engine.MaterialInstanceDynamic)
      (if (Variables|Default|GetIsMagic)
        (Rendering|Material|SetVectorParameterValue _returnvalue_4 "EmissionColor" (Variables|Default|GetCurrentRandomColor) :!class /Script/Engine.MaterialInstanceDynamic)
        (Rendering|Material|SetScalarParameterValue _returnvalue_4 "Emission" 1.5 :!class /Script/Engine.MaterialInstanceDynamic)))))

(event EventStartHovering
  (Rendering|Material|SetScalarParameterValue (Variables|Default|GetDispenserMaterial) "Emission" 0.025 :!class /Script/Engine.MaterialInstanceDynamic))

(fn ConstructionScript
  (Rendering|Components|TextRender|SetText (Variables|Default|GetNameText) (Variables|Default|GetDisplayName)))

(fn GetRandomColor
  (return (Class|KismetMathLibrary|HSVtoRGB (Math|Random|RandomFloatinRange 0.0 3.6e+02) 1.0 1.0 1.0)))