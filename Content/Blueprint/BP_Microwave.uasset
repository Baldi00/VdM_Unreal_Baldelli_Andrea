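; BP_Microwave is an interactable microwave prop that toggles on and off and highlights when hovered.
; BeginPlay creates a dynamic material instance on the mesh with a red base and emission color, and the hover events raise or clear its emission.
; Interact uses a FlipFlop to alternate between starting a stored 2D running sound and stopping it with an end sound, while setting the point light's visibility to match.
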(event EventStopHovering
  (Rendering|Material|SetScalarParameterValue (Variables|Default|GetMicrowaveMaterial) "Emission" 0.0 :!class /Script/Engine.MaterialInstanceDynamic))

(event EventBeginPlay
  (bind _returnvalue (Rendering|Material|CreateDynamicMaterialInstance (Variables|Default|GetMicrowave) 0 "/Game/Art/MaterialLibrary/M_DefaultMaterial.M_DefaultMaterial" "None" :!class /Script/Engine.PrimitiveComponent))
  (bind _output_get (Variables|Default|SetMicrowaveMaterial _returnvalue))
  (Rendering|Material|SetVectorParameterValue _output_get "BaseColor" "(R=0.791298,G=0.174647,B=0.174647,A=1.000000)" :!class /Script/Engine.MaterialInstanceDynamic)
  (Rendering|Material|SetVectorParameterValue _output_get "EmissionColor" "(R=0.791298,G=0.174647,B=0.174647,A=1.000000)" :!class /Script/Engine.MaterialInstanceDynamic))

(event EventInteract
  (bind _isa (Utilities|FlowControl|FlipFlop)
    (:A
      (bind _returnvalue (Audio|SpawnSound2D "/Game/Sounds/FX/MicrowaveRunning.MicrowaveRunning" 1.0 1.0 0.0 0))
      (Variables|Default|SetMicrowaveRunningSound _returnvalue))
    (:B
      (Audio|Components|Audio|Stop (Variables|Default|GetMicrowaveRunningSound))
      (Audio|PlaySound2D "/Game/Sounds/FX/MicrowaveEnd.MicrowaveEnd" 1.0 1.0 0.0 0 0)))
  (Rendering|SetVisibility (Variables|Default|GetPointLight) _isa false))

(event EventStartHovering
  (Rendering|Material|SetScalarParameterValue (Variables|Default|GetMicrowaveMaterial) "Emission" 0.025 :!class /Script/Engine.MaterialInstanceDynamic))

(fn ConstructionScript)