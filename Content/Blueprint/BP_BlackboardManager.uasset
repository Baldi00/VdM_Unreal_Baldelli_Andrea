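; Blackboard manager that lets the first-person player draw on and wipe a blackboard through a render target, cleared to black on BeginPlay.
; Each tick it polls the character's blackboard-hit and input flags, painting while interaction is pressed, otherwise clearing the whole board on right mouse.
; Painting converts the character's raycast hit to a UV, feeds it to a dynamic brush material, and draws that material into the render target.
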(event EventBeginPlay
  (Utilities|FlowControl|Sequence
    (:then_0
      (bind _returnvalue (Rendering|Material|CreateDynamicMaterialInstance "/Game/Art/MaterialLibrary/Blackboard/M_Blackboard_Brush.M_Blackboard_Brush" "None" "None" :!class /Script/Engine.KismetMaterialLibrary))
      (Variables|Default|SetBlackboardBrushMaterial _returnvalue))
    (:then_1
      (Rendering|ClearRenderTarget2D "/Game/Art/MaterialLibrary/Blackboard/RT_Blackboard.RT_Blackboard"))
    (:then_2
      (bind _asbp_first_person_character (Utilities|Casting|CastToBP_FirstPersonCharacter (Game|GetPlayerCharacter 0)))
      (Variables|Default|SetAs%20BP%20First%20Person%20Character _asbp_first_person_character))))

(event EventTick
  (params (DeltaSeconds :type Float%20%28single-precision%29))
  (if (Variables|/Game/FirstPerson/Blueprints/BP_FirstPersonCharacter.BP_FirstPersonCharacter_C|GetIsHittingBlackboard (Variables|Default|GetAs%20BP%20First%20Person%20Character))
    (if (Variables|/Game/FirstPerson/Blueprints/BP_FirstPersonCharacter.BP_FirstPersonCharacter_C|GetInteractionButtonPressed (Variables|Default|GetAs%20BP%20First%20Person%20Character))
      (|PaintToRenderTarget)
      (elif (Variables|/Game/FirstPerson/Blueprints/BP_FirstPersonCharacter.BP_FirstPersonCharacter_C|GetRightMousePressed (Variables|Default|GetAs%20BP%20First%20Person%20Character))
        (Rendering|ClearRenderTarget2D "/Game/Art/MaterialLibrary/Blackboard/RT_Blackboard.RT_Blackboard")))))

(fn ConstructionScript)