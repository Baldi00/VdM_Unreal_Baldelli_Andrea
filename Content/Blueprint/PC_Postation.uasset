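; PC_Postation is an interactable computer prop whose screens toggle on and off and whose case brightens slightly on hover.
; On BeginPlay it creates dynamic instances of M_Screen for the screen and case slots of SMPCPostation and caches the case's base color.
; Interact flip-flops the screen's emission and color between lit white and dark.
; StartHovering offsets the cached case color, and StopHovering restores it.
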(event EventStopHovering
  (Rendering|Material|SetVectorParameterValue (Variables|Default|GetCaseMaterial) "BaseColor" (Variables|Default|GetInitialCaseColor) :!class /Script/Engine.MaterialInstanceDynamic))

(event EventInteract
  (bind _screenmaterial (Variables|Default|GetScreenMaterial))
  (bind _screenmaterial_2 (Variables|Default|GetScreenMaterial))
  (Utilities|FlowControl|FlipFlop
    (:A
      (Rendering|Material|SetScalarParameterValue _screenmaterial_2 "Emission" 2.0 :!class /Script/Engine.MaterialInstanceDynamic)
      (Rendering|Material|SetVectorParameterValue _screenmaterial_2 "BaseColor" "(R=1.000000,G=1.000000,B=1.000000,A=1.000000)" :!class /Script/Engine.MaterialInstanceDynamic))
    (:B
      (Rendering|Material|SetScalarParameterValue _screenmaterial "Emission" 0.0 :!class /Script/Engine.MaterialInstanceDynamic)
      (Rendering|Material|SetVectorParameterValue _screenmaterial "BaseColor" "(R=0.000000,G=0.000000,B=0.000000,A=1.000000)" :!class /Script/Engine.MaterialInstanceDynamic))))

(event EventBeginPlay
  (bind _sm_pc_postation (Variables|Default|GetSM_PC_Postation))
  (Utilities|FlowControl|Sequence
    (:then_0
      (bind _returnvalue (Rendering|Material|CreateDynamicMaterialInstance "/Game/Art/MaterialLibrary/M_Screen.M_Screen" "None" "None" :!class /Script/Engine.KismetMaterialLibrary))
      (Variables|Default|SetScreenMaterial _returnvalue)
      (Rendering|Material|SetMaterial _sm_pc_postation 5 (Variables|Default|GetScreenMaterial))
      (Rendering|Material|SetMaterial _sm_pc_postation 13 (Variables|Default|GetScreenMaterial)))
    (:then_1
      (bind _returnvalue_2 (Rendering|Material|CreateDynamicMaterialInstance "/Game/Art/MaterialLibrary/M_Screen.M_Screen" "None" "None" :!class /Script/Engine.KismetMaterialLibrary))
      (bind _output_get (Variables|Default|SetCaseMaterial _returnvalue_2))
      (bind _returnvalue_3 (Rendering|Material|GetVectorParameterValue _output_get "BaseColor" :!class /Script/Engine.MaterialInstanceDynamic))
      (Variables|Default|SetInitialCaseColor _returnvalue_3)
      (Rendering|Material|SetMaterial (Variables|Default|GetSM_PC_Postation) 9 (Variables|Default|GetCaseMaterial)))))

(event EventStartHovering
  (Rendering|Material|SetVectorParameterValue (Variables|Default|GetCaseMaterial) "BaseColor" (+ (Variables|Default|GetInitialCaseColor) 0.025) :!class /Script/Engine.MaterialInstanceDynamic))

(fn ConstructionScript)